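; BP_Interactable is a switch-style object that turns linked BP_NonInteractable objects on or off.
; ToggleState loops over ConnectedObjects, casts each to BP_NonInteractable, calls SwitchOFF or SwitchON based on the current State, then flips that boolean.
; GetAttacked is an empty event, and nothing in this graph calls ToggleState.
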(event `ToggleState`
  (bind _connectedobjects (`self.ConnectedObjects`))
  (if (`self.State`)
    (for _array_element _connectedobjects
      (bind _asbp_non_interactable (cast `/Game/BP_Objects/BP_NonInteractable` _array_element))
      (`/Game/BP_Objects/I_SignalReciever.SwitchOFF` _asbp_non_interactable))
    (set `self.State` false)
    (else
      (for _array_element_2 _connectedobjects
        (bind _asbp_non_interactable_2 (cast `/Game/BP_Objects/BP_NonInteractable` _array_element_2))
        (`/Game/BP_Objects/I_SignalReciever.SwitchON` _asbp_non_interactable_2))
      (set `self.State` true))))

(event `GetAttacked`)

(fn `UserConstructionScript`)