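; BP_Pickable is a physics object that the player character can pick up and throw.
; GetAttacked acts as the pickup: if the player holds nothing, it disables collision and physics, snaps to the character's "pickableObject" mesh socket and registers as PickedObject.
; ThrowObject detaches it and restores physics and collision, without applying any impulse or clearing the character's PickedObject reference itself.
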(event `GetAttacked`
  (bind _mesh (`self.mesh`))
  (bind _asbp_third_person_character (cast `/Game/ThirdPerson/Blueprints/BP_ThirdPersonCharacter` (`GameplayStatics.GetPlayerPawn` 0)))
  (if (== (`/Game/ThirdPerson/Blueprints/BP_ThirdPersonCharacter.pickedObject` _asbp_third_person_character) null)
    (`PrimitiveComponent.SetCollisionEnabled` _mesh "NoCollision")
    (`PrimitiveComponent.SetSimulatePhysics` _mesh false)
    (`self.K2_AttachToComponent` (`Character.Mesh` _asbp_third_person_character) "pickableObject" "SnapToTarget" "SnapToTarget" "KeepWorld")
    (set `/Game/ThirdPerson/Blueprints/BP_ThirdPersonCharacter.pickedObject` self _asbp_third_person_character)))

(event `ThrowObject`
  (bind _mesh (`self.mesh`))
  (`self.K2_DetachFromActor` "KeepWorld" "KeepWorld" "KeepWorld")
  (`PrimitiveComponent.SetSimulatePhysics` _mesh true)
  (`PrimitiveComponent.SetCollisionEnabled` _mesh "QueryAndPhysics"))

(fn `UserConstructionScript`)