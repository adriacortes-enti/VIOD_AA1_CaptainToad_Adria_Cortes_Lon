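; AC_Health is a health component that tracks an HP value.
; On BeginPlay it binds handlers to the HealthAdd and HealthRemove dispatchers, then sets HP to MaxHP.
; Each add event raises HP by one while it is below MaxHP, and each remove event lowers it by one with no lower limit or death handling.
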(event `self.ReceiveBeginPlay`
  (add `self.HealthAdd` (delegate `AddHP`))
  (add `self.HealthRemove` (delegate `RemovHP`))
  (set `self.HP` (`self.MaxHP`)))

(event `AddHP`
  (if (< (`self.HP`) (`self.MaxHP`))
    (set `self.HP` (+ (`self.HP`) 1))))

(event `RemovHP`
  (set `self.HP` (- (`self.HP`) 1)))