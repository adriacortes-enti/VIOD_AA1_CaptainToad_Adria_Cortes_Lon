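; BP_RotatingBridge is a bridge actor that rotates around its vertical axis when switched on or off.
; SwitchON plays the Rotate timeline, whose track drives the actor's relative yaw.
; SwitchOFF plays a separate GoBack timeline the same way, but only when ShouldGoBack is set.
; A CanExecute flag blocks new switch events until the current rotation finishes.
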(event `/Game/BP_Objects/I_SignalReciever.SwitchON`
  (if (`self.canExecute`)
    (set `self.canExecute` false)
    (bind (_direction _newtrack_0) (`Timeline|Rotate` :!via `PlayFromStart`)
      (:`Update`
        (`self.K2_SetActorRelativeRotation` (`KismetMathLibrary.MakeRotator` 0.0 0.0 _newtrack_0)))
      (:`Finished`
        (set `self.canExecute` true)))))

(event `/Game/BP_Objects/I_SignalReciever.SwitchOFF`
  (if (and (`self.shouldGoBack`) (`self.canExecute`))
    (set `self.canExecute` false)
    (bind (_direction _newtrack_0) (`Timeline|GoBack` :!via `PlayFromStart`)
      (:`Update`
        (`self.K2_SetActorRelativeRotation` (`KismetMathLibrary.MakeRotator` 0.0 0.0 _newtrack_0)))
      (:`Finished`
        (set `self.canExecute` true)))))

(fn `UserConstructionScript`
  (`parent.UserConstructionScript`))