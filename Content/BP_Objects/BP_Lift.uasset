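; BP_Lift is a switchable lift actor that moves vertically in response to SwitchON and SwitchOFF events.
; Each event plays its own timeline from the start, GoUp or GoDown, whose track value sets the actor's absolute world Z with sweep, keeping current X and Y.
; CanExecute is cleared while a timeline runs and restored when it finishes, though neither event checks it here.
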(event `/Game/BP_Objects/I_SignalReciever.SwitchON`
  (bind (_returnvalue_x _returnvalue_y) (`KismetMathLibrary.BreakVector` (`self.K2_GetActorLocation`)))
  (set `self.canExecute` false)
  (bind (_direction _newtrack_0) (`Timeline|GoUp` :!via `PlayFromStart`)
    (:`Update`
      (`self.K2_SetActorLocation` (`KismetMathLibrary.MakeVector` _returnvalue_x _returnvalue_y _newtrack_0) true))
    (:`Finished`
      (set `self.canExecute` true))))

(event `/Game/BP_Objects/I_SignalReciever.SwitchOFF`
  (bind (_returnvalue_x _returnvalue_y) (`KismetMathLibrary.BreakVector` (`self.K2_GetActorLocation`)))
  (set `self.canExecute` false)
  (bind (_direction _newtrack_0) (`Timeline|GoDown` :!via `PlayFromStart`)
    (:`Update`
      (`self.K2_SetActorLocation` (`KismetMathLibrary.MakeVector` _returnvalue_x _returnvalue_y _newtrack_0) true))
    (:`Finished`
      (set `self.canExecute` true))))

(fn `UserConstructionScript`
  (`parent.UserConstructionScript`))