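; BP_Lock is a lock actor that opens for one designated key and switches on the objects linked to it.
; When that exact DesignedKey actor overlaps its Sphere, the lock destroys the key and clears PickedObject on the player's BP_ThirdPersonCharacter.
; It then calls SwitchON on every entry in ConnectedObjects, provided the character cast succeeds.
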(event `self.Sphere.OnComponentBeginOverlap`
  (params (OverlappedComponent :type "PrimitiveComponent Object Reference") (OtherActor :type "Actor Object Reference") (OtherComp :type "PrimitiveComponent Object Reference") (OtherBodyIndex :type Integer) (bFromSweep :type Boolean) (SweepResult :type "HitResult Structure (by ref)"))
  (if (== (`self.DesignedKey`) OtherActor)
    (`self.K2_DestroyActor` OtherActor)
    (bind _asbp_third_person_character (cast `/Game/ThirdPerson/Blueprints/BP_ThirdPersonCharacter` (`GameplayStatics.GetPlayerPawn` 0)))
    (set `/Game/ThirdPerson/Blueprints/BP_ThirdPersonCharacter.pickedObject` null _asbp_third_person_character)
    (for _array_element (`self.ConnectedObjects`)
      (`/Game/BP_Objects/I_SignalReciever.SwitchON` _array_element))))

(fn `UserConstructionScript`
  (`parent.UserConstructionScript`))